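; Combat component for BP_SumooCharacter that runs melee combos, aimed special projectiles, blocking and a bull rush.
; Data-driven attacks play montages whose notifies open combo queue windows and fire a one-shot socket sphere trace, hitting each character once.
; BPCResources gates attacks and rush by stamina, specials by mana.
; The rush launches forward, then drains stamina on Tick while repeatedly tracing and applying damage and knockback through ReceiveCombatHit.
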(event `self.ReceiveTick`
  (params (DeltaSeconds :type "Float (single-precision)"))
  (if (and (`self.RushIsActive`) (`self.IsRushing`))
    (`self.BullRushTick` DeltaSeconds)))

(event `StartAttack`
  (params (AttackIndex :type Integer))
  ; Attack
  (set `self.QueuedNextAttack` false)
  (set `self.CanQueueNextAttack` false)
  (bind _output_get (set `self.CurrentAttack` (`|GetArrayItem` (`self.AttackList`) AttackIndex)))
  (bind (_attackname _montage _startsection _damage _forwardknockback _upknockback _hittraceradius _cancombo _nextattackindex _staminacost _lockgroundmovement) (break `/Game/Sumoo/Data/ST_AttackData` _output_get))
  (`/Game/Sumoo/Blueprints/Characters/BP_SumooCharacter.TryLockMovement` (`self.OwnerCharacter`) _lockgroundmovement)
  (bind _notifyname (`|PlayMontage` (`self.OwnerMesh`) _montage 1.0 0.0 _attackname false)
    (:`OnCompleted`
      (`self.TryContinueCombo`))
    (:`OnNotifyBegin`
      (`self.HandleAttackNotifyBegin` _notifyname))
    (:`OnNotifyEnd`
      (`self.HandleAttackNotifyEnd` _notifyname))))

(event `ResetSpecialAttack`
  (`KismetSystemLibrary.Delay` 0.2)
  (set `self.CanSpecialAttack` true))

(fn `ApplyAttackHit`
  (bind _traceradius (`self.GetCurrentAttackTraceRadius`))
  (bind _outhits (`self.GetAttackTraceHits` _traceradius))
  (for _array_element _outhits
    (`self.TryApplyHitToCharacter` _array_element)))

(fn `ApplyHitEffects`
  (params (HitCharacter :type "/Game/Sumoo/Blueprints/Characters/BP_SumooCharacter Object Reference"))
  (bind _attackdamage (`self.GetCurrentAttackDamage`))
  (bind (_forwardknockback _upknockback) (`self.GetCurrentAttackKnockback`))
  (bind _asbp_sumoo_character (cast `/Game/Sumoo/Blueprints/Characters/BP_SumooCharacter` (`self.GetOwner`)))
  (`/Game/Sumoo/Blueprints/Characters/BP_SumooCharacter.ReceiveCombatHit` HitCharacter _attackdamage _asbp_sumoo_character _forwardknockback _upknockback))

(fn `ApplyRushHit`
  (params (HitCharacter :type "/Game/Sumoo/Blueprints/Characters/BP_SumooCharacter Object Reference"))
  (bind _asbp_sumoo_character (cast `/Game/Sumoo/Blueprints/Characters/BP_SumooCharacter` (`self.GetOwner`)))
  (`/Game/Sumoo/Blueprints/Characters/BP_SumooCharacter.ReceiveCombatHit` HitCharacter (`self.RushDamage`) _asbp_sumoo_character (`self.RushForwardKnockback`) (`self.RushUpKnockback`)))

(fn `ApplyRushMovement`
  (bind _ownercharacter (`self.OwnerCharacter`))
  (`Character.LaunchCharacter` _ownercharacter (* (`Actor.GetActorForwardVector` _ownercharacter) (`self.RushBurst`)) true false))

(fn `BullRushTick`
  (params (DeltaSeconds :type "Float (double-precision)"))
  (locals (StaminaCostThisFrame :type "Float (double-precision)"))
  (bind _resourcescomponent (`self.ResourcesComponent`))
  (if (> (`/Game/Sumoo/Blueprints/Components/BPC_Resources.CurrentStamina` _resourcescomponent) (* DeltaSeconds (`self.RushStaminaDrainPerSecond`)))
    (`/Game/Sumoo/Blueprints/Components/BPC_Resources.SpendStamina` _resourcescomponent (* DeltaSeconds (`self.RushStaminaDrainPerSecond`)))
    (bind _tracehits (`self.GetRushTraceHits`))
    (for _array_element _tracehits
      (bind _asbp_sumoo_character (cast `/Game/Sumoo/Blueprints/Characters/BP_SumooCharacter` (`.HitActor` (`GameplayStatics.BreakHitResult` _array_element))))
      (`self.ApplyRushHit` _asbp_sumoo_character))
    (else
      (`self.EndRush`))))

(fn `CanStartAttack`
  (params (AttackIndex :type Integer))
  (returns (CanAttackResult :type Boolean))
  (bind _ownercharacter (`self.OwnerCharacter`))
  (bind _staminacost (`self.GetAttackStaminaCost` AttackIndex))
  (return (and (>= (`/Game/Sumoo/Blueprints/Components/BPC_Resources.CurrentStamina` (`self.ResourcesComponent`)) _staminacost) (not (`/Game/Sumoo/Blueprints/Characters/BP_SumooCharacter.IsStunned` _ownercharacter)) (not (`/Game/Sumoo/Blueprints/Characters/BP_SumooCharacter.IsDodging` _ownercharacter)) (not (`/Game/Sumoo/Blueprints/Characters/BP_SumooCharacter.IsAiming` _ownercharacter)) (`self.CanAttack`))))

(fn `CanStartRush`
  (returns (CanStartRush :type Boolean))
  (bind _ownercharacter (`self.OwnerCharacter`))
  (return (and (`self.CanRush`) (not (`self.IsRushing`)) (not (`self.IsAttacking`)) (not (`self.IsBlocking`)) (not (`/Game/Sumoo/Blueprints/Characters/BP_SumooCharacter.IsStunned` _ownercharacter)) (not (`/Game/Sumoo/Blueprints/Characters/BP_SumooCharacter.IsDodging` _ownercharacter)) (`/Game/Sumoo/Blueprints/Characters/BP_SumooCharacter.CanMove` _ownercharacter) (>= (`/Game/Sumoo/Blueprints/Components/BPC_Resources.CurrentStamina` (`self.ResourcesComponent`)) (`self.RushStaminaCost`)))))

(fn `CanStartSpecialAttack`
  (params (`Special Attack Index` :type Integer))
  (returns (CanSpecialAttack :type Boolean) (ManaCost :type "Float (double-precision)"))
  (bind _ownercharacter (`self.OwnerCharacter`))
  (bind _manacost (`self.GetSpecialAttackManaCost` `Special Attack Index`))
  (return (and (>= (`/Game/Sumoo/Blueprints/Components/BPC_Resources.CurrentMana` (`self.ResourcesComponent`)) _manacost) (not (`/Game/Sumoo/Blueprints/Characters/BP_SumooCharacter.IsDodging` _ownercharacter)) (not (`/Game/Sumoo/Blueprints/Characters/BP_SumooCharacter.IsAttacking` _ownercharacter)) (`/Game/Sumoo/Blueprints/Characters/BP_SumooCharacter.IsAiming` _ownercharacter)) _manacost))

(fn `CommitAttack`
  (params (AttackIndex :type Integer))
  (bind _staminacost (`self.GetAttackStaminaCost` AttackIndex))
  (`/Game/Sumoo/Blueprints/Components/BPC_Resources.SpendStamina` (`/Game/Sumoo/Blueprints/Characters/BP_SumooCharacter.BPC_Resources` (`self.OwnerCharacter`)) _staminacost)
  (set `self.IsAttacking` true)
  (`self.StartAttack` AttackIndex))

(fn `EndRush`
  (`self.ResetRush`))

(fn `GetAttackLaunchVelocity`
  (params (HitCharacter :type "Character Object Reference") (Direction :type "Vector Structure"))
  (returns (ReturnValue :type "Vector Structure"))
  (return (0.0 0.0 0.0)))

(fn `GetAttackStaminaCost`
  (params (AttackIndex :type Integer))
  (returns (StaminaCost :type "Float (double-precision)"))
  (return (`.StaminaCost_24_C16AAF6A4391B4198A3510BA70732E01` (break `/Game/Sumoo/Data/ST_AttackData` (`|GetArrayItem` (`self.AttackList`) AttackIndex)))))

(fn `GetAttackTraceHits`
  (params (TraceRadius :type "Float (double-precision)"))
  (returns (OutHits :type "Array of HitResult Structure"))
  (bind (_startlocation _endlocation) (`self.GetAttackTracePostions`))
  (bind _outhits (`KismetSystemLibrary.SphereTraceMulti` :`Start` _startlocation :`End` _endlocation :`Radius` TraceRadius :`TraceChannel` "TraceTypeQuery1" :`bTraceComplex` true :`DrawDebugType` "ForDuration" :`DrawTime` 2.0))
  (return _outhits))

(fn `GetAttackTracePostions`
  (returns (StartLocation :type "Vector Structure") (EndLocation :type "Vector Structure"))
  (bind _returnvalue (`SceneComponent.GetSocketLocation` (`self.OwnerMesh`) (`.HitSocketName_34_3A134EB4431F87ADFC1FC49BECA390DB` (break `/Game/Sumoo/Data/ST_AttackData` (`self.CurrentAttack`)))))
  (bind _output_get (set `self.PreviousHitSocketLocaiton` _returnvalue))
  (return (`self.PreviousHitSocketLocaiton`) _output_get))

(fn `GetCurrentAttackCanCombo`
  (returns (CanCombo :type Boolean))
  (return (`.CanCombo_18_EDC5E62B446775EEC33456AEA3E4FE9F` (break `/Game/Sumoo/Data/ST_AttackData` (`self.CurrentAttack`)))))

(fn `GetCurrentAttackDamage`
  (returns (AttackDamage :type "Float (double-precision)"))
  (return (`.Damage_11_79C1A2014A6F41070310CBBD2480ED29` (break `/Game/Sumoo/Data/ST_AttackData` (`self.CurrentAttack`)))))

(fn `GetCurrentAttackKnockback`
  (returns (ForwardKnockback :type "Float (double-precision)") (UpKnockback :type "Float (double-precision)"))
  (bind (_attackname _montage _startsection _damage _forwardknockback _upknockback) (break `/Game/Sumoo/Data/ST_AttackData` (`self.CurrentAttack`)))
  (return _forwardknockback _upknockback))

(fn `GetCurrentAttackNextIndex`
  (returns (Index :type Integer))
  (return (`.NextAttackIndex_21_47BBB5CD4619E6300CEFFA95060AE2B8` (break `/Game/Sumoo/Data/ST_AttackData` (`self.CurrentAttack`)))))

(fn `GetCurrentAttackTraceRadius`
  (returns (TraceRadius :type "Float (double-precision)"))
  (return (`.HitTraceRadius_15_9C06E3774528477531E013AF8D7DB092` (break `/Game/Sumoo/Data/ST_AttackData` (`self.CurrentAttack`)))))

(fn `GetRushTraceHits`
  (returns (TraceHits :type "Array of HitResult Structure"))
  (bind _ownercharacter (`self.OwnerCharacter`))
  (bind _ownercharacter_2 (`self.OwnerCharacter`))
  (bind _outhits (`KismetSystemLibrary.SphereTraceMulti` :`Start` (+ (`Actor.K2_GetActorLocation` _ownercharacter_2) (* (`SceneComponent.GetForwardVector` (`Actor.RootComponent` _ownercharacter_2)) 60.0)) :`End` (+ (`Actor.K2_GetActorLocation` _ownercharacter) (* (`SceneComponent.GetForwardVector` (`Actor.RootComponent` _ownercharacter)) 140.0)) :`Radius` (`self.RushTraceRadius`) :`TraceChannel` "TraceTypeQuery1" :`bTraceComplex` true :`DrawDebugType` "ForDuration" :`DrawTime` 2.0))
  (return _outhits))

(fn `GetSpecialAttackManaCost`
  (params (SpecialAttackIndex :type Integer))
  (returns (ManaCost :type "Float (double-precision)"))
  (return (`.ManaCost_7_BB377DFA4E8904D9AD1938B994CD0874` (break `/Game/Sumoo/Data/ST_SpecialAttackData` (`|GetArrayItem` (`self.SpecialAttackList`) SpecialAttackIndex)))))

(fn `HandleAttackLanding`
  (if (`self.IsAttacking`)
    (if (`.LockGroundMovement_30_0EF0C2C94F3DCB15E7F2BD9BEF4A9107` (break `/Game/Sumoo/Data/ST_AttackData` (`self.CurrentAttack`)))
      (set `/Game/Sumoo/Blueprints/Characters/BP_SumooCharacter.CanMove` false (`self.OwnerCharacter`)))))

(fn `HandleAttackNotifyBegin`
  (params (NotifyName :type Name))
  (if (== NotifyName "AttackActive")
    (`KismetArrayLibrary.Array_Clear` (`self.HitCharactersThisAttack`))
    (set `self.AttackIsActive` true)
    (`self.ApplyAttackHit`)
    (elif (== NotifyName "ComboWindow")
      (bind _cancombo (`self.GetCurrentAttackCanCombo`))
      (if _cancombo
        (set `self.CanQueueNextAttack` true)))))

(fn `HandleAttackNotifyEnd`
  (params (NotifyName :type Name)))

(fn `HandleBlockLanding`
  (if (`self.IsBlocking`)
    (set `/Game/Sumoo/Blueprints/Characters/BP_SumooCharacter.CanMove` false (`self.OwnerCharacter`))))

(fn `InitializeCombat`
  (bind _asbp_sumoo_character (cast `/Game/Sumoo/Blueprints/Characters/BP_SumooCharacter` (`self.GetOwner`)))
  (set `self.OwnerCharacter` _asbp_sumoo_character)
  (set `self.OwnerMesh` (`Character.Mesh` _asbp_sumoo_character))
  (set `self.OwnerMovement` (`Character.CharacterMovement` _asbp_sumoo_character))
  (set `self.ResourcesComponent` (`/Game/Sumoo/Blueprints/Characters/BP_SumooCharacter.BPC_Resources` _asbp_sumoo_character)))

(fn `ResetAttackState`
  (set `self.IsAttacking` false)
  (set `self.QueuedNextAttack` false)
  (set `self.CanQueueNextAttack` false)
  (set `/Game/Sumoo/Blueprints/Characters/BP_SumooCharacter.CanMove` true (`self.OwnerCharacter`)))

(fn `ResetRush`
  (set `self.IsRushing` false)
  (set `self.CanRush` true)
  (set `self.RushIsActive` false))

(fn `ResetSpecialAttackState`
  (set `self.CanSpecialAttack` true))

(fn `SpawnProjectile`
  (bind _ownercharacter (`self.OwnerCharacter`))
  (`|SpawnActorFromClass` "/Game/Sumoo/Blueprints/BP_SpecialProjectile.BP_SpecialProjectile_C" (`KismetMathLibrary.MakeTransform` (+ (+ (`Actor.K2_GetActorLocation` _ownercharacter) (* (`Actor.GetActorForwardVector` _ownercharacter) 100.0)) (0.0 0.0 60.0)) (`Controller.GetControlRotation` (`Pawn.GetController` _ownercharacter))) "Undefined" "MultiplyWithRoot" _ownercharacter (`self.CurrentSpecialAttack`) _ownercharacter)
  (set `self.IsAttacking` false)
  (`self.ResetSpecialAttack`))

(fn `StartBlock`
  (set `self.IsBlocking` true)
  (set `self.CanAttack` false)
  (if (not (`NavMovementComponent.IsFalling` (`self.OwnerMovement`)))
    (set `/Game/Sumoo/Blueprints/Characters/BP_SumooCharacter.CanMove` false (`self.OwnerCharacter`))))

(fn `StartRush`
  (set `self.IsRushing` true)
  (set `self.RushIsActive` true)
  (set `self.CanRush` false)
  (`/Game/Sumoo/Blueprints/Components/BPC_Resources.SpendStamina` (`self.ResourcesComponent`) (`self.RushStaminaCost`))
  (`self.ApplyRushMovement`)
  (`self.BullRushTick` 0.0))

(fn `StopBlock`
  (set `self.IsBlocking` false)
  (set `/Game/Sumoo/Blueprints/Characters/BP_SumooCharacter.CanMove` true (`self.OwnerCharacter`))
  (set `self.CanAttack` true))

(fn `TryApplyHitToCharacter`
  (params (HitResult :type "HitResult Structure"))
  (bind _asbp_sumoo_character (cast `/Game/Sumoo/Blueprints/Characters/BP_SumooCharacter` (`.HitActor` (`GameplayStatics.BreakHitResult` HitResult))))
  (if (`KismetArrayLibrary.Array_Contains` (`self.HitCharactersThisAttack`))
    _
    (elif (not (`/Game/Sumoo/Blueprints/Characters/BP_SumooCharacter.IsInvulnerable` _asbp_sumoo_character))
      (`KismetArrayLibrary.Array_Add` (`self.HitCharactersThisAttack`) _asbp_sumoo_character)
      (`self.ApplyHitEffects` _asbp_sumoo_character))))

(fn `TryAttack`
  (params (AttackIndex :type Integer))
  (if (`self.IsAttacking`)
    (`self.TryQueueCombo`)
    (else
      (bind _canattackresult (`self.CanStartAttack` AttackIndex))
      (if _canattackresult
        (`self.CommitAttack` AttackIndex)))))

(fn `TryContinueCombo`
  (if (`self.QueuedNextAttack`)
    (bind _cancombo (`self.GetCurrentAttackCanCombo`))
    (if _cancombo
      (bind _index (`self.GetCurrentAttackNextIndex`))
      (bind _staminacost (`self.GetAttackStaminaCost` _index))
      (if (>= (`/Game/Sumoo/Blueprints/Components/BPC_Resources.CurrentStamina` (`/Game/Sumoo/Blueprints/Characters/BP_SumooCharacter.BPC_Resources` (`self.OwnerCharacter`))) _staminacost)
        (set `self.CanQueueNextAttack` false)
        (set `self.QueuedNextAttack` false)
        (bind _index_2 (`self.GetCurrentAttackNextIndex`))
        (`self.CommitAttack` _index_2)
        (else
          (`self.ResetAttackState`)))
      (else
        (`self.ResetAttackState`)))
    (else
      (`self.ResetAttackState`))))

(fn `TryQueueCombo`
  (if (`self.CanQueueNextAttack`)
    (if (not (`self.QueuedNextAttack`))
      (set `self.QueuedNextAttack` true)
      (set `self.PendingAttackIndex` (`.NextAttackIndex_21_47BBB5CD4619E6300CEFFA95060AE2B8` (break `/Game/Sumoo/Data/ST_AttackData` (`self.CurrentAttack`)))))))

(fn `TryRush`
  (bind _canstartrush (`self.CanStartRush`))
  (if _canstartrush
    (`self.StartRush`)))

(fn `TrySpecialAttack`
  (params (SpecialAttackIndex :type Integer))
  (if (`self.CanSpecialAttack`)
    (set `self.CurrentSpecialAttack` (`|GetArrayItem` (`self.SpecialAttackList`) SpecialAttackIndex))
    (bind (_canspecialattack _manacost) (`self.CanStartSpecialAttack` SpecialAttackIndex))
    (if _canspecialattack
      (`/Game/Sumoo/Blueprints/Components/BPC_Resources.SpendMana` (`self.ResourcesComponent`) _manacost)
      (set `self.IsAttacking` true)
      (set `self.CanSpecialAttack` false)
      (`self.SpawnProjectile`))))