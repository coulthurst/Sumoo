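; BPC_Resources is an actor component that tracks stamina and mana pools.
; Regen functions add a rate scaled by delta seconds and spend functions subtract a cost, each clamping the result between zero and the maximum.
; It does not drive regeneration itself, as BeginPlay is empty and Tick is disabled.
; HasEnoughStamina and HasEnoughMana are empty stubs with no logic yet.
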(event `self.ReceiveBeginPlay`)

(fn `HasEnoughMana`)

(fn `HasEnoughStamina`)

(fn `RegenMana`
  (params (DeltaSeconds :type "Float (double-precision)"))
  (set `self.CurrentMana` (`KismetMathLibrary.FClamp` (+ (`self.CurrentMana`) (* DeltaSeconds (`self.ManaRegenRate`))) 0.0 (`self.MaxMana`))))

(fn `RegenStamina`
  (params (DeltaSeconds :type "Float (double-precision)"))
  (set `self.CurrentStamina` (`KismetMathLibrary.FClamp` (+ (`self.CurrentStamina`) (* DeltaSeconds (`self.StaminaRegenRate`))) 0.0 (`self.MaxStamina`))))

(fn `SpendMana`
  (params (ManaCost :type "Float (double-precision)"))
  (set `self.CurrentMana` (`KismetMathLibrary.FClamp` (- (`self.CurrentMana`) ManaCost) 0.0 (`self.MaxMana`))))

(fn `SpendStamina`
  (params (StaminaCost :type "Float (double-precision)"))
  (set `self.CurrentStamina` (`KismetMathLibrary.FClamp` (- (`self.CurrentStamina`) StaminaCost) 0.0 (`self.MaxStamina`))))