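; BP_SumooCharacter_AI_Walk is a Sumoo AI character that walks toward player character 0.
; Each Tick, unless stunned, it feeds GetDirection into movement input and snaps its rotation to face the player on the horizontal plane.
; It also tests attack range and cooldown, but that branch triggers nothing in this graph.
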(event `self.ReceiveTick`
  (params (DeltaSeconds :type "Float (single-precision)"))
  (bind _returnvalue (`GameplayStatics.GetPlayerCharacter` 0))
  (bind _returnvalue_2 (`self.K2_GetActorLocation`))
  (if (not (`self.IsStunned`))
    (bind _hitdirection (`self.GetDirection` _returnvalue))
    (`self.AddMovementInput` _hitdirection)
    (`self.K2_SetActorRotation` (`KismetMathLibrary.FindLookAtRotation` _returnvalue_2 (`KismetMathLibrary.MakeVector` (.x (`self.K2_GetActorLocation` _returnvalue)) (.y (`self.K2_GetActorLocation` _returnvalue)) (.z _returnvalue_2))))
    (if (and (< (`self.GetDistanceTo` _returnvalue) (`self.AIAttackRange`)) (not (`self.IsAIAttackOnCooldown`)))
      _)))

(fn `UserConstructionScript`
  (`parent.UserConstructionScript`))