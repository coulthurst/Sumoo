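; Sumoo game mode that handles ring-outs, stock loss and respawning for characters.
; A ring-out clears other characters' lock-on to the victim, hides it, then removes a stock behind dead/respawning guards.
; With stocks left, it immediately teleports to the first PlayerStart found, resets damage and state, and gets timed invulnerability.
; Elimination calls DisableCharacter, which is an empty stub, as is the uncalled CheckForWinner.
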(event `StartRespawnInvulnerability`
  (params (RespawnCharacter :type "/Game/Sumoo/Blueprints/Characters/BP_SumooCharacter Object Reference"))
  (`KismetSystemLibrary.Delay` (`self.RespawnInvulnerabilityTimer`))
  (set `/Game/Sumoo/Blueprints/Characters/BP_SumooCharacter.IsInvulnerable` false RespawnCharacter))

(fn `CheckForWinner`)

(fn `DisableCharacter`
  (params (DisabledCharacter :type "/Game/Sumoo/Blueprints/Characters/BP_SumooCharacter Object Reference")))

(fn `DisableLockOn`
  (params (RingOutCharacter :type "/Game/Sumoo/Blueprints/Characters/BP_SumooCharacter Object Reference"))
  (bind _outactors (`GameplayStatics.GetAllActorsOfClass` "/Game/Sumoo/Blueprints/Characters/BP_SumooCharacter.BP_SumooCharacter_C"))
  (for _array_element _outactors
    (if (== (`/Game/Sumoo/Blueprints/Characters/BP_SumooCharacter.LockedTarget` _array_element) RingOutCharacter)
      (`/Game/Sumoo/Blueprints/Characters/BP_SumooCharacter.DisableLockOn` _array_element))))

(fn `HandleRingOut`
  (params (RingOutCharacter :type "/Game/Sumoo/Blueprints/Characters/BP_SumooCharacter Object Reference"))
  (`self.DisableLockOn` RingOutCharacter)
  (`self.SetActorHiddenInGame` RingOutCharacter true)
  (if (`/Game/Sumoo/Blueprints/Characters/BP_SumooCharacter.IsRespawning` RingOutCharacter)
    _
    (elif (`KismetSystemLibrary.IsValid` RingOutCharacter)
      (if (not (or (`/Game/Sumoo/Blueprints/Characters/BP_SumooCharacter.IsDead` RingOutCharacter) (`/Game/Sumoo/Blueprints/Characters/BP_SumooCharacter.IsRespawning` RingOutCharacter)))
        (`self.ReduceStock` RingOutCharacter)))))

(fn `ReduceStock`
  (params (`Ring Out Character` :type "/Game/Sumoo/Blueprints/Characters/BP_SumooCharacter Object Reference"))
  (set `/Game/Sumoo/Blueprints/Characters/BP_SumooCharacter.IsDead` true `Ring Out Character`)
  (set `/Game/Sumoo/Blueprints/Characters/BP_SumooCharacter.IsLockedOn` false `Ring Out Character`)
  (set `/Game/Sumoo/Blueprints/Characters/BP_SumooCharacter.IsRespawning` true `Ring Out Character`)
  (set `/Game/Sumoo/Blueprints/Characters/BP_SumooCharacter.CanMove` false `Ring Out Character`)
  (set `/Game/Sumoo/Blueprints/Characters/BP_SumooCharacter.RemainingStocks` (- (`/Game/Sumoo/Blueprints/Characters/BP_SumooCharacter.RemainingStocks` `Ring Out Character`) 1) `Ring Out Character`)
  (`self.SetActorEnableCollision` `Ring Out Character` false)
  (`self.TryRespawnCharacter` `Ring Out Character`))

(fn `ResetForRespawn`
  (params (RespawnCharacter :type "/Game/Sumoo/Blueprints/Characters/BP_SumooCharacter Object Reference"))
  (set `/Game/Sumoo/Blueprints/Characters/BP_SumooCharacter.DamagePercent` 0.0 RespawnCharacter)
  (set `/Game/Sumoo/Blueprints/Characters/BP_SumooCharacter.CanMove` true RespawnCharacter)
  (set `/Game/Sumoo/Blueprints/Characters/BP_SumooCharacter.IsDead` false RespawnCharacter)
  (set `/Game/Sumoo/Blueprints/Characters/BP_SumooCharacter.IsRespawning` false RespawnCharacter)
  (set `/Game/Sumoo/Blueprints/Characters/BP_SumooCharacter.IsInvulnerable` true RespawnCharacter)
  (`self.SetActorHiddenInGame` RespawnCharacter false)
  (`self.SetActorEnableCollision` RespawnCharacter true)
  (`self.StartRespawnInvulnerability` RespawnCharacter))

(fn `RespawnCharacter`
  (params (RespawnCharacter :type "/Game/Sumoo/Blueprints/Characters/BP_SumooCharacter Object Reference"))
  (if (`KismetSystemLibrary.IsValid` RespawnCharacter)
    (`self.TeleportRespawnCharacter` RespawnCharacter)
    (`self.ResetForRespawn` RespawnCharacter)))

(fn `TeleportRespawnCharacter`
  (params (RespawnCharacter :type "/Game/Sumoo/Blueprints/Characters/BP_SumooCharacter Object Reference"))
  (bind _outactors (`GameplayStatics.GetAllActorsOfClass` "/Script/Engine.PlayerStart"))
  (`self.K2_SetActorTransform` RespawnCharacter (`self.GetTransform` (`|GetArrayItem` _outactors)) false false)
  (`MovementComponent.StopMovementImmediately` (`Character.CharacterMovement` RespawnCharacter)))

(fn `TryRespawnCharacter`
  (params (`Ring Out Character` :type "/Game/Sumoo/Blueprints/Characters/BP_SumooCharacter Object Reference"))
  (if (> (`/Game/Sumoo/Blueprints/Characters/BP_SumooCharacter.RemainingStocks` `Ring Out Character`) 0)
    (`self.RespawnCharacter` `Ring Out Character`)
    (else
      (`self.DisableCharacter` `Ring Out Character`))))

(fn `UserConstructionScript`)