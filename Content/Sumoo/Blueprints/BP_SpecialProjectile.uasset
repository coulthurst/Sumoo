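; BP_SpecialProjectile is the projectile for a Sumoo character's special attack.
; When it overlaps a Sumoo character other than its owner, it applies a special hit.
; The hit passes damage and forward and upward knockback from SpecialAttackData to the target's ReceiveCombatHit, crediting the instigator as attacker, then destroys the projectile.
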(event `self.ReceiveActorBeginOverlap`
  (params (OtherActor :type "Actor Object Reference"))
  (bind _asbp_sumoo_character (cast `/Game/Sumoo/Blueprints/Characters/BP_SumooCharacter` OtherActor))
  (if (!= _asbp_sumoo_character (`self.GetOwner`))
    (`self.ApplySpecialHit` _asbp_sumoo_character)))

(fn `ApplySpecialHit`
  (params (`Hit Character` :type "/Game/Sumoo/Blueprints/Characters/BP_SumooCharacter Object Reference"))
  (bind (_attackname _projectileclass _manacost _damage _forwardknockback _upknockback) (break `/Game/Sumoo/Data/ST_SpecialAttackData` (`self.SpecialAttackData`)))
  (`/Game/Sumoo/Blueprints/Characters/BP_SumooCharacter.ReceiveCombatHit` `Hit Character` _damage (cast `/Game/Sumoo/Blueprints/Characters/BP_SumooCharacter` (`self.Instigator`) :!pure true) _forwardknockback _upknockback)
  (`self.K2_DestroyActor`))

(fn `UserConstructionScript`)